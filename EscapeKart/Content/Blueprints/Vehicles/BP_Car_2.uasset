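; BP_Car_2 is a vehicle Blueprint that switches four particle effects on and off with driving speed.
; Each tick it checks the vehicle movement component's forward speed and activates the particle systems above a small threshold, deactivating them otherwise.
; Tick also runs a short downward visibility trace from the mesh, but its result is unused.
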(event `self.ReceiveTick`
  (params (DeltaSeconds :type "Float (single-precision)"))
  (bind _particlesystem1 (`self.ParticleSystem1`))
  (bind _returnvalue (`SceneComponent.K2_GetComponentLocation` (`self.Mesh`)))
  (`KismetSystemLibrary.LineTraceSingle` _returnvalue (- _returnvalue (0.0 0.0 150.0)) "TraceTypeQuery1")
  (if (> (`WheeledVehicleMovementComponent.GetForwardSpeed` (`self.VehicleMovement`)) 10.0)
    (`ActorComponent.SetActive` _particlesystem1 true false)
    (`ActorComponent.SetActive` (`self.ParticleSystem`) true false)
    (`ActorComponent.SetActive` (`self.ParticleSystem3`) true false)
    (`ActorComponent.SetActive` (`self.ParticleSystem2`) true false)
    (else
      (`ActorComponent.SetActive` _particlesystem1 false false)
      (`ActorComponent.SetActive` (`self.ParticleSystem`) false false)
      (`ActorComponent.SetActive` (`self.ParticleSystem3`) false false)
      (`ActorComponent.SetActive` (`self.ParticleSystem2`) false false))))

(fn `UserConstructionScript`)