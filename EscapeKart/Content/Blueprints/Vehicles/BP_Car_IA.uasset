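; BP_Car_IA is an AI-driven car that follows the spline of its ActivePath at a constant half throttle set on BeginPlay.
; Each Tick, GetPath projects a fixed distance ahead along the nearest spline tangent and snaps that point back onto the spline as a look-ahead target.
; The yaw difference between the car's heading and that target is mapped to a clamped steering input for VehicleMovement.
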(event `self.ReceiveBeginPlay`
  (`WheeledVehicleMovementComponent.SetThrottleInput` (`self.VehicleMovement`) 0.5))

(event `self.ReceiveTick`
  (params (DeltaSeconds :type "Float (single-precision)"))
  (bind _sterring (`self.GetPath`))
  (`WheeledVehicleMovementComponent.SetSteeringInput` (`self.VehicleMovement`) _sterring))

(fn `GetPath`
  (returns (Sterring :type "Float (double-precision)"))
  (bind _returnvalue (`self.K2_GetActorLocation`))
  (bind _spline (`/Game/Blueprints/Vehicles/Path.Spline` (`self.ActivePath`)))
  (bind (_returnvalue_roll _returnvalue_pitch _returnvalue_yaw) (`KismetMathLibrary.BreakRotator` (`KismetMathLibrary.NormalizedDeltaRotator` (`KismetMathLibrary.FindLookAtRotation` _returnvalue (`SplineComponent.FindLocationClosestToWorldLocation` _spline (+ (* (`KismetMathLibrary.Normal` (`SplineComponent.FindTangentClosestToWorldLocation` _spline _returnvalue "World")) 200.0) _returnvalue) "World")) (`self.K2_GetActorRotation`))))
  (return (`KismetMathLibrary.MapRangeClamped` _returnvalue_yaw -90.0 90.0 -1.0 1.0)))

(fn `UserConstructionScript`)